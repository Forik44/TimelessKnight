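; Riddle scanner that sends an activate message to a locked door once its trigger has been occupied for five seconds.
; Each overlap restarts the scan sound or effect, a timeline that moves the scanner toward UpState, and a retriggerable delay.
; An overlap counter detects when the trigger empties, then clears the triggered flag, stops the scan, resets the scanner position and deactivates the door message.
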(event `self.Trigger.OnActorBeginOverlap`
  (params (OverlappedActor :type "Actor Object Reference") (OtherActor :type "Actor Object Reference"))
  (bind _scan (`self.Scan`))
  (`|ExecutionSequence`
    (:`then_0`
      (set `self.Triggered` true)
      (`|ExecutionSequence`
        (:`then_0`
          (`AudioComponent.Stop` _scan)
          (`AudioComponent.Play` _scan 0.0)
          (`KismetSystemLibrary.RetriggerableDelay` 5.0)
          (if (`self.Triggered`)
            (`AudioComponent.Stop` _scan)
            (message `/Game/Blueprint/BP_Interaction.Activate` (`self.LockedDoor`))))
        (:`then_1`
          (bind (_direction _lerp) (`Timeline|ScanerAnimation` :!via `PlayFromStart` :!label _label)
            (:`Update`
              (`SceneComponent.K2_SetRelativeLocation` (`self.Scanner`) (`KismetMathLibrary.VLerp` (0.0 0.0 0.0) (`self.UpState`) _lerp) false false))
            (:`Finished`
              (`SceneComponent.K2_SetWorldLocation` (`self.Scanner`) (0.0 0.0 0.0) false false))))))
    (:`then_1`
      (bind _result (`/Engine/EditorBlueprintResources/StandardMacros.IncrementInt` (`self.CountActors`))
        (:`  `
          (set `self.CountActors` _result))))))

(event `self.ReceiveBeginPlay`
  (`|ExecutionSequence`
    (:`then_0`
      (set `self.Triggered` false))
    (:`then_1`
      (set `self.CountActors` 0))
    (:`then_2`
      (`AudioComponent.Stop` (`self.Scan`)))))

(event `self.Trigger.OnActorEndOverlap`
  (params (OverlappedActor :type "Actor Object Reference") (OtherActor :type "Actor Object Reference"))
  (bind _result (`/Engine/EditorBlueprintResources/StandardMacros.DecrementInt` (`self.CountActors`))
    (:`  `
      (if (== (`self.CountActors`) 0)
        (set `self.Triggered` false)
        (`|ExecutionSequence`
          (:`then_0`
            (goto _label :!via `Stop`))
          (:`then_1`
            (`SceneComponent.K2_SetWorldLocation` (`self.Scanner`) (0.0 0.0 0.0) false false))
          (:`then_2`
            (`AudioComponent.Stop` (`self.Scan`))
            (message `/Game/Blueprint/BP_Interaction.Deactivate` (`self.LockedDoor`))))))))

(fn `UserConstructionScript`)