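; BP_FastEnemyCharacter is the fast enemy character, holding its AI setup and sound controls.
; On BeginPlay it sets mode and type on its DefaulAIController, then silences its step, run-step, idle/default, scream and attack audio; a failed controller cast skips both.
; Small functions play footsteps or toggle default, scream, attack and crawl sounds, with no callers in this graph.
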(event `self.ReceiveBeginPlay`
  (bind _asdefaul_aicontroller (cast `/Game/AI/Controller/DefaulAIController` (`AIBlueprintHelperLibrary.GetAIController` self)))
  (`/Game/AI/Controller/DefaulAIController.SetAiModeAndType` _asdefaul_aicontroller false 1)
  (`AudioComponent.Stop` (`self.Step`))
  (`AudioComponent.Stop` (`self.Default`))
  (`AudioComponent.Stop` (`self.Scream`))
  (`AudioComponent.Stop` (`self.RunStep`))
  (`AudioComponent.Stop` (`self.Attack`)))

(fn `PlayRunStepSound`
  (`AudioComponent.Play` (`self.RunStep`) 0.0))

(fn `PlayStepSound`
  (`AudioComponent.Play` (`self.Step`) 0.0))

(fn `SetPlayAttackSound`
  (params (isPlay :type Boolean))
  (if isPlay
    (`AudioComponent.Play` (`self.Attack`) 0.3)
    (else
      (`AudioComponent.Stop` (`self.Attack`)))))

(fn `SetPlayCrawlSound`
  (params (isPlay :type Boolean))
  (if isPlay
    (`AudioComponent.Play` (`self.Crawl`) 0.0)
    (else
      (`AudioComponent.Stop` (`self.Crawl`)))))

(fn `SetPlayDefaultSound`
  (params (isPlay :type Boolean))
  (if isPlay
    (`AudioComponent.Play` (`self.Default`) 0.0)
    (else
      (`AudioComponent.Stop` (`self.Default`)))))

(fn `SetPlayScreamSound`
  (params (isPlay :type Boolean))
  (if isPlay
    (`AudioComponent.Play` (`self.Scream`) -0.5)
    (else
      (`AudioComponent.Stop` (`self.Scream`)))))

(fn `UserConstructionScript`)