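; Falling ceiling riddle trap that, once activated, messages a locked door and, after a short delay, drops five ceiling sections in sequence.
; Chained timelines lerp each section between up and down positions in order 4, 3, 2, 1, 5, flagging only the moving one as damaging.
; Hits from sections 1-4 deal heavy damage to an FPCharacter unless its time system is reversing.
; Section 5's damage logic is disconnected.
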(event `self.ReceiveBeginPlay`
  (set `self.IsActivate` false))

(event `/Game/Blueprint/BP_Interaction.Activate`
  (if (not (`self.IsActivate`))
    (set `self.IsActivate` true)
    (message `/Game/Blueprint/BP_Interaction.Activate` (`self.LockedDoor`))
    (`KismetSystemLibrary.Delay` 1.0)
    (set `self.IsDamage4` true)
    (bind (_direction _lerp) (`Timeline|FallAnimation4`)
      (:`Update`
        (`SceneComponent.K2_SetRelativeLocation` (`self.Ceil4`) (`KismetMathLibrary.VLerp` (`self.UpState4`) (`self.DownState4`) _lerp) false false))
      (:`Finished`
        (set `self.IsDamage4` false)
        (set `self.IsDamage3` true)
        (bind (_direction_2 _lerp_2) (`Timeline|FallAnimation3`)
          (:`Update`
            (`SceneComponent.K2_SetRelativeLocation` (`self.Ceil3`) (`KismetMathLibrary.VLerp` (`self.UpState3`) (`self.DownState3`) _lerp_2) false false))
          (:`Finished`
            (set `self.IsDamage3` false)
            (set `self.IsDamage2` true)
            (bind (_direction_3 _lerp_3) (`Timeline|FallAnimation2`)
              (:`Update`
                (`SceneComponent.K2_SetRelativeLocation` (`self.Ceil2`) (`KismetMathLibrary.VLerp` (`self.UpState2`) (`self.DownState2`) _lerp_3) false false))
              (:`Finished`
                (set `self.IsDamage2` false)
                (set `self.IsDamage1` true)
                (bind (_direction_4 _lerp_4) (`Timeline|FallAnimation`)
                  (:`Update`
                    (`SceneComponent.K2_SetRelativeLocation` (`self.Ceil`) (`KismetMathLibrary.VLerp` (`self.UpState`) (`self.DownState`) _lerp_4) false false))
                  (:`Finished`
                    (set `self.IsDamage1` false)
                    (set `self.IsDamage5` true)
                    (bind (_direction_5 _lerp_5) (`Timeline|FallAnimation5`)
                      (:`Update`
                        (`SceneComponent.K2_SetRelativeLocation` (`self.Ceil5`) (`KismetMathLibrary.VLerp` (`self.UpState5`) (`self.DownState5`) _lerp_5) false false))
                      (:`Finished`
                        (set `self.IsDamage5` false)))))))))))))

(event `self.Ceil.OnComponentHit`
  (params (HitComponent :type "PrimitiveComponent Object Reference") (OtherActor :type "Actor Object Reference") (OtherComp :type "PrimitiveComponent Object Reference") (NormalImpulse :type "Vector Structure") (Hit :type "HitResult Structure (by ref)"))
  (if (`self.IsDamage1`)
    (bind _asfpcharacter (cast `FPCharacter` OtherActor))
    (bind _returnvalue (`TimeSystemCharacterComponent.GetIsReverse` (`FPCharacter.TimeSystemCharacter` _asfpcharacter)))
    (if (not _returnvalue)
      (`GameplayStatics.ApplyDamage` OtherActor 200.0 null self))))

(event `self.Ceil2.OnComponentHit`
  (params (HitComponent :type "PrimitiveComponent Object Reference") (OtherActor :type "Actor Object Reference") (OtherComp :type "PrimitiveComponent Object Reference") (NormalImpulse :type "Vector Structure") (Hit :type "HitResult Structure (by ref)"))
  (if (`self.IsDamage2`)
    (bind _asfpcharacter (cast `FPCharacter` OtherActor))
    (bind _returnvalue (`TimeSystemCharacterComponent.GetIsReverse` (`FPCharacter.TimeSystemCharacter` _asfpcharacter)))
    (if (not _returnvalue)
      (`GameplayStatics.ApplyDamage` OtherActor 200.0 null self))))

(event `self.Ceil3.OnComponentHit`
  (params (HitComponent :type "PrimitiveComponent Object Reference") (OtherActor :type "Actor Object Reference") (OtherComp :type "PrimitiveComponent Object Reference") (NormalImpulse :type "Vector Structure") (Hit :type "HitResult Structure (by ref)"))
  (if (`self.IsDamage3`)
    (bind _asfpcharacter (cast `FPCharacter` OtherActor))
    (bind _returnvalue (`TimeSystemCharacterComponent.GetIsReverse` (`FPCharacter.TimeSystemCharacter` _asfpcharacter)))
    (if (not _returnvalue)
      (`GameplayStatics.ApplyDamage` OtherActor 200.0 null self))))

(event `self.Ceil4.OnComponentHit`
  (params (HitComponent :type "PrimitiveComponent Object Reference") (OtherActor :type "Actor Object Reference") (OtherComp :type "PrimitiveComponent Object Reference") (NormalImpulse :type "Vector Structure") (Hit :type "HitResult Structure (by ref)"))
  (if (`self.IsDamage4`)
    (bind _asfpcharacter (cast `FPCharacter` OtherActor))
    (bind _returnvalue (`TimeSystemCharacterComponent.GetIsReverse` (`FPCharacter.TimeSystemCharacter` _asfpcharacter)))
    (if (not _returnvalue)
      (`GameplayStatics.ApplyDamage` OtherActor 200.0 null self))))

(event `self.Ceil5.OnComponentHit`
  (params (HitComponent :type "PrimitiveComponent Object Reference") (OtherActor :type "Actor Object Reference") (OtherComp :type "PrimitiveComponent Object Reference") (NormalImpulse :type "Vector Structure") (Hit :type "HitResult Structure (by ref)")))

(fn `UserConstructionScript`)