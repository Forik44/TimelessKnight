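; Button is an interactable riddle Blueprint that toggles another actor on and off.
; Each Interact flips IsActive and sends an Activate or Deactivate message to ActorToActivate.
; The ButtonLerp timeline plays forward or in reverse, sliding the button component between its zero relative location and SecondState.
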(event `self.ReceiveBeginPlay`
  (set `self.IsActive` false))

(event `/Game/Blueprint/BP_Interaction.Interact`
  (if (`self.IsActive`)
    (message `/Game/Blueprint/BP_Interaction.Deactivate` (`self.ActorToActivate`))
    (set `self.IsActive` false)
    (bind (_direction _lerp) (`Timeline|ButtonLerp` :!via `Reverse` :!label _label)
      (:`Update`
        (`SceneComponent.K2_SetRelativeLocation` (`self.Button`) (`KismetMathLibrary.VLerp` (0.0 0.0 0.0) (`self.SecondState`) _lerp) false false)))
    (else
      (message `/Game/Blueprint/BP_Interaction.Activate` (`self.ActorToActivate`))
      (set `self.IsActive` true)
      (goto _label))))

(fn `UserConstructionScript`)