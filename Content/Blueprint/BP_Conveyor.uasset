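; Conveyor belt that carries overlapping actors along the mesh's forward vector, reversing when Rewinding is set.
; Construction builds a dynamic track material from color, arrow scale and speed; Tick feeds it a wrapped ArtificialTime so scrolling follows the rewind direction.
; Characters get swept offsets, with CanControl/Controlling flags arbitrating between overlapping conveyors so only one pushes.
; An FPCharacter that jumps or falls while controlled inherits the belt velocity.
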(event `self.ReceiveTick`
  (params (DeltaSeconds :type "Float (single-precision)"))
  (bind _returnvalue (`KismetMathLibrary.GetForwardVector` (`SceneComponent.K2_GetComponentRotation` (`self.StaticMesh`))))
  (bind _returnvalue_2 (+ (* (`KismetMathLibrary.Conv_BoolToInt` (`self.Rewinding`)) -2) 1))
  (bind _returnvalue_3 (* _returnvalue_2 (`self.Speed`)))
  (bind _returnvalue_4 (+ (* _returnvalue_2 DeltaSeconds) (`self.ArtificialTime`)))
  (bind _returnvalue_5 (* _returnvalue (* DeltaSeconds _returnvalue_3)))
  (bind _output_get (set `self.ArtificialTime` (- _returnvalue_4 (* (`KismetMathLibrary.FFloor` (/ _returnvalue_4 (`self.Track Revolve Time`))) (`self.Track Revolve Time`)))))
  (`MaterialInstanceDynamic.SetScalarParameterValue` (`self.Track`) "ArtificialTime" _output_get)
  (set `self.CanControl` true)
  (for _array_element (`PrimitiveComponent.GetOverlappingActors` (`self.Box`) null)
    (bind _ascharacter (cast `Character` _array_element)
      (:`then`
        (set `self.Character` _ascharacter))
      (:`CastFailed`
        (bind _asbp_conveyor (cast `/Game/Blueprint/BP_Conveyor` _array_element)
          (:`then`
            (if (or (and (`PrimitiveComponent.IsOverlappingActor` (`/Game/Blueprint/BP_Conveyor.Box` _asbp_conveyor) (`self.Character`)) (`/Game/Blueprint/BP_Conveyor.CanControl` _asbp_conveyor)) (`/Game/Blueprint/BP_Conveyor.Controlling` _asbp_conveyor))
              (set `self.CanControl` false)))
          (:`CastFailed`
            (`self.K2_AddActorWorldOffset` _array_element _returnvalue_5 false false))))))
  (bind _asfpcharacter (cast `FPCharacter` (`self.Character`)))
  (if (`self.CanControl`)
    (bind _charactermovement (`Character.CharacterMovement` _asfpcharacter))
    (if (and (or (`Character.bWasJumping` _asfpcharacter) (`NavMovementComponent.IsFalling` _charactermovement)) (`self.Controlling`))
      (set `MovementComponent.Velocity` (+ (`MovementComponent.Velocity` _charactermovement) (* _returnvalue _returnvalue_3)) _charactermovement)
      (set `self.CanControl` false)
      (set `self.Controlling` false :!label _label)
      (else
        (set `self.Controlling` true)
        (if (`PrimitiveComponent.IsOverlappingActor` (`self.Box`) (`self.Character`))
          (`self.K2_AddActorWorldOffset` (`self.Character`) _returnvalue_5 true false)
          (set `self.CanControl` (`PrimitiveComponent.IsOverlappingActor` (`self.Box`) (`self.Character`)))
          (else
            (goto _label)))))))

(fn `UserConstructionScript`
  (bind _staticmesh (`self.StaticMesh`))
  (bind _returnvalue (* (* (`self.Speed`) (`self.Track Speed`)) (.x (`SceneComponent.K2_GetComponentScale` (`self.StaticMesh`))) 0.5))
  (bind _returnvalue_2 (`PrimitiveComponent.CreateDynamicMaterialInstance` _staticmesh 0 null "None"))
  (set `self.Track` _returnvalue_2)
  (`PrimitiveComponent.SetMaterial` _staticmesh 0 _returnvalue_2)
  (`MaterialInstanceDynamic.SetVectorParameterValue` _returnvalue_2 "Color" (`self.Color`))
  (`MaterialInstanceDynamic.SetScalarParameterValue` _returnvalue_2 "X Scale" (`self.Arrow Scale`))
  (set `self.Track Revolve Time` (/ 1.0 (`KismetMathLibrary.Abs` _returnvalue)))
  (`MaterialInstanceDynamic.SetScalarParameterValue` _returnvalue_2 "X Speed" _returnvalue))