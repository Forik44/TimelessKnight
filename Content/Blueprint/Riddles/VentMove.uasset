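; VentMove is a riddle Blueprint for a vent that moves once when the player interacts with it.
; The first Interact sets IsActive, which blocks any later triggers since nothing resets it after BeginPlay.
; A timeline then blends the Vent component's relative transform from FirstState to SecondState without sweeping for collision.
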(event `self.ReceiveBeginPlay`
  (set `self.IsActive` false))

(event `/Game/Blueprint/BP_Interaction.Interact`
  (if (not (`self.IsActive`))
    (set `self.IsActive` true)
    (bind (_direction _lerp) (`Timeline|Timeline_0`)
      (:`Update`
        (`SceneComponent.K2_SetRelativeTransform` (`self.Vent`) (`KismetMathLibrary.TLerp` (`self.FirstState`) (`self.SecondState`) _lerp) false false)))))

(fn `UserConstructionScript`)