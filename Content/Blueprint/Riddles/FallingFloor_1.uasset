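; FallingFloor_1 is a puzzle floor piece whose four columns drop after a capsule component enters its Box trigger.
; Begin overlap arms a trigger flag and counts occupants, then waits through a short retriggerable delay before checking the flag.
; End overlap decrements the count and clears the flag at zero, cancelling a pending drop.
; Four timelines lerp the columns from up to down positions, with no logic to raise them again.
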(event `self.ReceiveBeginPlay`
  (set `self.Triggered` false))

(event `self.Box.OnComponentBeginOverlap`
  (params (OverlappedComponent :type "PrimitiveComponent Object Reference") (OtherActor :type "Actor Object Reference") (OtherComp :type "PrimitiveComponent Object Reference") (OtherBodyIndex :type Integer) (bFromSweep :type Boolean) (SweepResult :type "HitResult Structure (by ref)"))
  (cast `CapsuleComponent` OtherComp)
  (`|ExecutionSequence`
    (:`then_0`
      (set `self.Triggered` true)
      (`KismetSystemLibrary.RetriggerableDelay` 0.5)
      (if (`self.Triggered`)
        (`|ExecutionSequence`
          (:`then_0`
            (bind (_direction _lerp) (`Timeline|Timeline_3`)
              (:`Update`
                (`SceneComponent.K2_SetRelativeLocation` (`self.Colomn4`) (`KismetMathLibrary.VLerp` (`self.UpState`) (`self.DownState`) _lerp) false false))))
          (:`then_1`
            (bind (_direction_2 _lerp_2) (`Timeline|Timeline_2`)
              (:`Update`
                (`SceneComponent.K2_SetRelativeLocation` (`self.Colomn3`) (`KismetMathLibrary.VLerp` (`self.UpState1`) (`self.DownState1`) _lerp_2) false false))))
          (:`then_2`
            (bind (_direction_3 _lerp_3) (`Timeline|Timeline_1`)
              (:`Update`
                (`SceneComponent.K2_SetRelativeLocation` (`self.Colomn2`) (`KismetMathLibrary.VLerp` (`self.UpState2`) (`self.DownState2`) _lerp_3) false false))))
          (:`then_3`
            (bind (_direction_4 _lerp_4) (`Timeline|Timeline_0`)
              (:`Update`
                (`SceneComponent.K2_SetRelativeLocation` (`self.Colomn1`) (`KismetMathLibrary.VLerp` (`self.UpState3`) (`self.DownState3`) _lerp_4) false false)))))))
    (:`then_1`
      (bind _result (`/Engine/EditorBlueprintResources/StandardMacros.IncrementInt` (`self.CountActors`))
        (:`  `
          (set `self.CountActors` _result))))))

(event `self.Box.OnComponentEndOverlap`
  (params (OverlappedComponent :type "PrimitiveComponent Object Reference") (OtherActor :type "Actor Object Reference") (OtherComp :type "PrimitiveComponent Object Reference") (OtherBodyIndex :type Integer))
  (cast `CapsuleComponent` OtherComp)
  (bind _result (`/Engine/EditorBlueprintResources/StandardMacros.DecrementInt` (`self.CountActors`))
    (:`  `
      (if (== (`self.CountActors`) 0)
        (set `self.Triggered` false)))))

(fn `UserConstructionScript`)