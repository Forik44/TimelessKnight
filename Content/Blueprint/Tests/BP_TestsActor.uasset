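; Test actor that smoke-tests the player's FPCharacter stat setters when play begins, reporting results through PrintString.
; FPCharacterTest runs four sequenced blocks, each calling a setter, reading the value back and printing whether it equals the expected, often clamped, value.
; Only the ChangeMana block exercises mana; the blocks labelled ChaneHP, TakeDamage and Pop all call ChangeXP, with TakeDamage expecting a floor of 1 instead of 0 for negative inputs.
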(event `self.ReceiveBeginPlay`
  (`KismetSystemLibrary.PrintString` "DriverCreated")
  (`self.FPCharacter Test`))

(fn `FPCharacter Test`
  (bind _asfpcharacter (cast `FPCharacter` (`GameplayStatics.GetPlayerCharacter` 0) :!pure true))
  (bind _asfpcharacter_2 (cast `FPCharacter` (`GameplayStatics.GetPlayerCharacter` 0) :!pure true))
  (bind _asfpcharacter_3 (cast `FPCharacter` (`GameplayStatics.GetPlayerCharacter` 0) :!pure true))
  (bind _asfpcharacter_4 (cast `FPCharacter` (`GameplayStatics.GetPlayerCharacter` 0) :!pure true))
  (bind _asfpcharacter_5 (cast `FPCharacter` (`GameplayStatics.GetPlayerCharacter` 0) :!pure true))
  (bind _asfpcharacter_6 (cast `FPCharacter` (`GameplayStatics.GetPlayerCharacter` 0) :!pure true))
  (bind _asfpcharacter_7 (cast `FPCharacter` (`GameplayStatics.GetPlayerCharacter` 0) :!pure true))
  (bind _asfpcharacter_8 (cast `FPCharacter` (`GameplayStatics.GetPlayerCharacter` 0) :!pure true))
  (bind _asfpcharacter_9 (cast `FPCharacter` (`GameplayStatics.GetPlayerCharacter` 0) :!pure true))
  (bind _asfpcharacter_10 (cast `FPCharacter` (`GameplayStatics.GetPlayerCharacter` 0) :!pure true))
  (bind _asfpcharacter_11 (cast `FPCharacter` (`GameplayStatics.GetPlayerCharacter` 0) :!pure true))
  (bind _asfpcharacter_12 (cast `FPCharacter` (`GameplayStatics.GetPlayerCharacter` 0) :!pure true))
  (bind _asfpcharacter_13 (cast `FPCharacter` (`GameplayStatics.GetPlayerCharacter` 0) :!pure true))
  (bind _asfpcharacter_14 (cast `FPCharacter` (`GameplayStatics.GetPlayerCharacter` 0) :!pure true))
  (bind _asfpcharacter_15 (cast `FPCharacter` (`GameplayStatics.GetPlayerCharacter` 0) :!pure true))
  (bind _asfpcharacter_16 (cast `FPCharacter` (`GameplayStatics.GetPlayerCharacter` 0) :!pure true))
  (bind _asfpcharacter_17 (cast `FPCharacter` (`GameplayStatics.GetPlayerCharacter` 0) :!pure true))
  (bind _asfpcharacter_18 (cast `FPCharacter` (`GameplayStatics.GetPlayerCharacter` 0) :!pure true))
  (bind _asfpcharacter_19 (cast `FPCharacter` (`GameplayStatics.GetPlayerCharacter` 0) :!pure true))
  (bind _asfpcharacter_20 (cast `FPCharacter` (`GameplayStatics.GetPlayerCharacter` 0) :!pure true))
  (bind _asfpcharacter_21 (cast `FPCharacter` (`GameplayStatics.GetPlayerCharacter` 0) :!pure true))
  (bind _asfpcharacter_22 (cast `FPCharacter` (`GameplayStatics.GetPlayerCharacter` 0) :!pure true))
  (bind _asfpcharacter_23 (cast `FPCharacter` (`GameplayStatics.GetPlayerCharacter` 0) :!pure true))
  (bind _asfpcharacter_24 (cast `FPCharacter` (`GameplayStatics.GetPlayerCharacter` 0) :!pure true))
  (bind _asfpcharacter_25 (cast `FPCharacter` (`GameplayStatics.GetPlayerCharacter` 0) :!pure true))
  (bind _asfpcharacter_26 (cast `FPCharacter` (`GameplayStatics.GetPlayerCharacter` 0) :!pure true))
  (bind _asfpcharacter_27 (cast `FPCharacter` (`GameplayStatics.GetPlayerCharacter` 0) :!pure true))
  (bind _asfpcharacter_28 (cast `FPCharacter` (`GameplayStatics.GetPlayerCharacter` 0) :!pure true))
  (bind _asfpcharacter_29 (cast `FPCharacter` (`GameplayStatics.GetPlayerCharacter` 0) :!pure true))
  (bind _asfpcharacter_30 (cast `FPCharacter` (`GameplayStatics.GetPlayerCharacter` 0) :!pure true))
  (bind _asfpcharacter_31 (cast `FPCharacter` (`GameplayStatics.GetPlayerCharacter` 0) :!pure true))
  (bind _asfpcharacter_32 (cast `FPCharacter` (`GameplayStatics.GetPlayerCharacter` 0) :!pure true))
  (`|ExecutionSequence`
    (:`then_0`
      (`KismetSystemLibrary.PrintString` "ChaneHP")
      (`FPCharacter.ChangeXP` _asfpcharacter_11 10.0)
      (bind _returnvalue (`FPCharacter.GetXP` _asfpcharacter_11))
      (`KismetSystemLibrary.PrintString` (`KismetStringLibrary.Concat_StrStr` "1)" (`KismetStringLibrary.Conv_BoolToString` (== 10.0 _returnvalue))))
      (`FPCharacter.ChangeXP` _asfpcharacter_12 90.0)
      (bind _returnvalue_2 (`FPCharacter.GetXP` _asfpcharacter_12))
      (`KismetSystemLibrary.PrintString` (`KismetStringLibrary.Concat_StrStr` "2)" (`KismetStringLibrary.Conv_BoolToString` (== 90.0 _returnvalue_2))))
      (`FPCharacter.ChangeXP` _asfpcharacter_13 110.0)
      (bind _returnvalue_3 (`FPCharacter.GetXP` _asfpcharacter_13))
      (`KismetSystemLibrary.PrintString` (`KismetStringLibrary.Concat_StrStr` "3)" (`KismetStringLibrary.Conv_BoolToString` (== _returnvalue_3 100.0))))
      (`FPCharacter.ChangeXP` _asfpcharacter_14 -10.0)
      (bind _returnvalue_4 (`FPCharacter.GetXP` _asfpcharacter_14))
      (`KismetSystemLibrary.PrintString` (`KismetStringLibrary.Concat_StrStr` "4)" (`KismetStringLibrary.Conv_BoolToString` (== _returnvalue_4 0.0))))
      (`FPCharacter.ChangeXP` _asfpcharacter_15 0.0)
      (bind _returnvalue_5 (`FPCharacter.GetXP` _asfpcharacter_15))
      (`KismetSystemLibrary.PrintString` (`KismetStringLibrary.Concat_StrStr` "5)" (`KismetStringLibrary.Conv_BoolToString` (== 0.0 _returnvalue_5))))
      (`FPCharacter.ChangeXP` _asfpcharacter_16 100.0)
      (bind _returnvalue_6 (`FPCharacter.GetXP` _asfpcharacter_16))
      (`KismetSystemLibrary.PrintString` (`KismetStringLibrary.Concat_StrStr` "6)" (`KismetStringLibrary.Conv_BoolToString` (== 100.0 _returnvalue_6))))
      (`FPCharacter.ChangeXP` _asfpcharacter_18 15.5)
      (bind _returnvalue_7 (`FPCharacter.GetXP` _asfpcharacter_18))
      (`KismetSystemLibrary.PrintString` (`KismetStringLibrary.Concat_StrStr` "7)" (`KismetStringLibrary.Conv_BoolToString` (== 15.5 _returnvalue_7))))
      (`FPCharacter.ChangeXP` _asfpcharacter_19 -6876867.0)
      (bind _returnvalue_8 (`FPCharacter.GetXP` _asfpcharacter_19))
      (`KismetSystemLibrary.PrintString` (`KismetStringLibrary.Concat_StrStr` "8)" (`KismetStringLibrary.Conv_BoolToString` (== 0.0 _returnvalue_8))))
      (`KismetSystemLibrary.PrintString` "Hello")
      (`KismetSystemLibrary.PrintString` "Hello")
      (`KismetSystemLibrary.PrintString` "Hello"))
    (:`then_1`
      (`KismetSystemLibrary.PrintString` "ChangeMana")
      (`FPCharacter.ChangeMana` _asfpcharacter_2 90.0)
      (bind _returnvalue_9 (`FPCharacter.GetMana` _asfpcharacter_2))
      (`KismetSystemLibrary.PrintString` (`KismetStringLibrary.Concat_StrStr` "1)" (`KismetStringLibrary.Conv_BoolToString` (== 90.0 _returnvalue_9))))
      (`FPCharacter.ChangeMana` _asfpcharacter_3 30.299999)
      (bind _returnvalue_10 (`FPCharacter.GetMana` _asfpcharacter_3))
      (`KismetSystemLibrary.PrintString` (`KismetStringLibrary.Concat_StrStr` "2)" (`KismetStringLibrary.Conv_BoolToString` (== 30.299999 _returnvalue_10))))
      (`FPCharacter.ChangeMana` _asfpcharacter_4 220.0)
      (bind _returnvalue_11 (`FPCharacter.GetMana` _asfpcharacter_4))
      (`KismetSystemLibrary.PrintString` (`KismetStringLibrary.Concat_StrStr` "3)" (`KismetStringLibrary.Conv_BoolToString` (== _returnvalue_11 200.0))))
      (`FPCharacter.ChangeMana` _asfpcharacter_5 -10.0)
      (bind _returnvalue_12 (`FPCharacter.GetMana` _asfpcharacter_5))
      (`KismetSystemLibrary.PrintString` (`KismetStringLibrary.Concat_StrStr` "4)" (`KismetStringLibrary.Conv_BoolToString` (== _returnvalue_12 0.0))))
      (`FPCharacter.ChangeMana` _asfpcharacter_7 0.0)
      (bind _returnvalue_13 (`FPCharacter.GetMana` _asfpcharacter_7))
      (`KismetSystemLibrary.PrintString` (`KismetStringLibrary.Concat_StrStr` "5)" (`KismetStringLibrary.Conv_BoolToString` (== 0.0 _returnvalue_13))))
      (`FPCharacter.ChangeMana` _asfpcharacter_8 200.0)
      (bind _returnvalue_14 (`FPCharacter.GetMana` _asfpcharacter_8))
      (`KismetSystemLibrary.PrintString` (`KismetStringLibrary.Concat_StrStr` "6)" (`KismetStringLibrary.Conv_BoolToString` (== 200.0 _returnvalue_14))))
      (`FPCharacter.ChangeMana` _asfpcharacter_9 123.456001)
      (bind _returnvalue_15 (`FPCharacter.GetMana` _asfpcharacter_9))
      (`KismetSystemLibrary.PrintString` (`KismetStringLibrary.Concat_StrStr` "7)" (`KismetStringLibrary.Conv_BoolToString` (== 123.456001 _returnvalue_15))))
      (`FPCharacter.ChangeMana` _asfpcharacter_10 -6876867.0)
      (bind _returnvalue_16 (`FPCharacter.GetMana` _asfpcharacter_10))
      (`KismetSystemLibrary.PrintString` (`KismetStringLibrary.Concat_StrStr` "8)" (`KismetStringLibrary.Conv_BoolToString` (== _returnvalue_16 0.0))))
      (`KismetSystemLibrary.PrintString` "Hello")
      (`KismetSystemLibrary.PrintString` "Hello")
      (`KismetSystemLibrary.PrintString` "Hello"))
    (:`then_2`
      (`KismetSystemLibrary.PrintString` "TakeDamage")
      (`FPCharacter.ChangeXP` _asfpcharacter_20 10.0)
      (bind _returnvalue_17 (`FPCharacter.GetXP` _asfpcharacter_20))
      (`KismetSystemLibrary.PrintString` (`KismetStringLibrary.Concat_StrStr` "1)" (`KismetStringLibrary.Conv_BoolToString` (== 10.0 _returnvalue_17))))
      (`FPCharacter.ChangeXP` _asfpcharacter_21 90.0)
      (bind _returnvalue_18 (`FPCharacter.GetXP` _asfpcharacter_21))
      (`KismetSystemLibrary.PrintString` (`KismetStringLibrary.Concat_StrStr` "2)" (`KismetStringLibrary.Conv_BoolToString` (== 90.0 _returnvalue_18))))
      (`FPCharacter.ChangeXP` _asfpcharacter_22 110.0)
      (bind _returnvalue_19 (`FPCharacter.GetXP` _asfpcharacter_22))
      (`KismetSystemLibrary.PrintString` (`KismetStringLibrary.Concat_StrStr` "3)" (`KismetStringLibrary.Conv_BoolToString` (== _returnvalue_19 100.0))))
      (`FPCharacter.ChangeXP` _asfpcharacter_23 -10.0)
      (bind _returnvalue_20 (`FPCharacter.GetXP` _asfpcharacter_23))
      (`KismetSystemLibrary.PrintString` (`KismetStringLibrary.Concat_StrStr` "4)" (`KismetStringLibrary.Conv_BoolToString` (== _returnvalue_20 1.0))))
      (`FPCharacter.ChangeXP` _asfpcharacter_24 0.0)
      (bind _returnvalue_21 (`FPCharacter.GetXP` _asfpcharacter_24))
      (`KismetSystemLibrary.PrintString` (`KismetStringLibrary.Concat_StrStr` "5)" (`KismetStringLibrary.Conv_BoolToString` (== 0.0 _returnvalue_21))))
      (`FPCharacter.ChangeXP` _asfpcharacter_25 100.0)
      (bind _returnvalue_22 (`FPCharacter.GetXP` _asfpcharacter_25))
      (`KismetSystemLibrary.PrintString` (`KismetStringLibrary.Concat_StrStr` "6)" (`KismetStringLibrary.Conv_BoolToString` (== 100.0 _returnvalue_22))))
      (`FPCharacter.ChangeXP` _asfpcharacter_26 15.5)
      (bind _returnvalue_23 (`FPCharacter.GetXP` _asfpcharacter_26))
      (`KismetSystemLibrary.PrintString` (`KismetStringLibrary.Concat_StrStr` "7)" (`KismetStringLibrary.Conv_BoolToString` (== 15.5 _returnvalue_23))))
      (`FPCharacter.ChangeXP` _asfpcharacter_27 -6876867.0)
      (bind _returnvalue_24 (`FPCharacter.GetXP` _asfpcharacter_27))
      (`KismetSystemLibrary.PrintString` (`KismetStringLibrary.Concat_StrStr` "8)" (`KismetStringLibrary.Conv_BoolToString` (== 1.0 _returnvalue_24))))
      (`KismetSystemLibrary.PrintString` "Hello")
      (`KismetSystemLibrary.PrintString` "Hello")
      (`KismetSystemLibrary.PrintString` "Hello"))
    (:`then_3`
      (`KismetSystemLibrary.PrintString` "Pop")
      (`FPCharacter.ChangeXP` _asfpcharacter_32 10.0)
      (bind _returnvalue_25 (`FPCharacter.GetXP` _asfpcharacter_32))
      (`KismetSystemLibrary.PrintString` (`KismetStringLibrary.Concat_StrStr` "1)" (`KismetStringLibrary.Conv_BoolToString` (== 10.0 _returnvalue_25))))
      (`FPCharacter.ChangeXP` _asfpcharacter_6 90.0)
      (bind _returnvalue_26 (`FPCharacter.GetXP` _asfpcharacter_6))
      (`KismetSystemLibrary.PrintString` (`KismetStringLibrary.Concat_StrStr` "2)" (`KismetStringLibrary.Conv_BoolToString` (== 90.0 _returnvalue_26))))
      (`FPCharacter.ChangeXP` _asfpcharacter_17 110.0)
      (bind _returnvalue_27 (`FPCharacter.GetXP` _asfpcharacter_17))
      (`KismetSystemLibrary.PrintString` (`KismetStringLibrary.Concat_StrStr` "3)" (`KismetStringLibrary.Conv_BoolToString` (== _returnvalue_27 100.0))))
      (`FPCharacter.ChangeXP` _asfpcharacter_28 -10.0)
      (bind _returnvalue_28 (`FPCharacter.GetXP` _asfpcharacter_28))
      (`KismetSystemLibrary.PrintString` (`KismetStringLibrary.Concat_StrStr` "4)" (`KismetStringLibrary.Conv_BoolToString` (== _returnvalue_28 0.0))))
      (`FPCharacter.ChangeXP` _asfpcharacter_29 0.0)
      (bind _returnvalue_29 (`FPCharacter.GetXP` _asfpcharacter_29))
      (`KismetSystemLibrary.PrintString` (`KismetStringLibrary.Concat_StrStr` "5)" (`KismetStringLibrary.Conv_BoolToString` (== 0.0 _returnvalue_29))))
      (`FPCharacter.ChangeXP` _asfpcharacter_30 100.0)
      (bind _returnvalue_30 (`FPCharacter.GetXP` _asfpcharacter_30))
      (`KismetSystemLibrary.PrintString` (`KismetStringLibrary.Concat_StrStr` "6)" (`KismetStringLibrary.Conv_BoolToString` (== 100.0 _returnvalue_30))))
      (`FPCharacter.ChangeXP` _asfpcharacter_31 15.5)
      (bind _returnvalue_31 (`FPCharacter.GetXP` _asfpcharacter_31))
      (`KismetSystemLibrary.PrintString` (`KismetStringLibrary.Concat_StrStr` "7)" (`KismetStringLibrary.Conv_BoolToString` (== 15.5 _returnvalue_31))))
      (`FPCharacter.ChangeXP` _asfpcharacter -6876867.0)
      (bind _returnvalue_32 (`FPCharacter.GetXP` _asfpcharacter))
      (`KismetSystemLibrary.PrintString` (`KismetStringLibrary.Concat_StrStr` "8)" (`KismetStringLibrary.Conv_BoolToString` (== 0.0 _returnvalue_32))))
      (`KismetSystemLibrary.PrintString` "Hello")
      (`KismetSystemLibrary.PrintString` "Hello")
      (`KismetSystemLibrary.PrintString` "Hello"))))

(fn `UserConstructionScript`)