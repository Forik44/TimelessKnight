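; A fire barrel interactive item that explodes and triggers falling-floor, platform and vent actors.
; When its activation type matches, an FPCharacter entering the sphere calls Explosion.
; Explosion activates the fire effect, adds an audio component, fires a radial force impulse and destroys the barrel.
; It then sends activate messages to the linked FallingFloor, Platform and Vent, after the destroy call.
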(event `self.Sphere.OnComponentBeginOverlap`
  (params (OverlappedComponent :type "PrimitiveComponent Object Reference") (OtherActor :type "Actor Object Reference") (OtherComp :type "PrimitiveComponent Object Reference") (OtherBodyIndex :type Integer) (bFromSweep :type Boolean) (SweepResult :type "HitResult Structure (by ref)"))
  (switch `int` (`self.TypeAcivate`)
    (:`1`
      (cast `FPCharacter` OtherActor)
      (`self.Explosion`))))

(fn `Explosion`
  (`ActorComponent.Activate` (`self.Fire`) false)
  (`AddComponent|NODE_AddAudioComponent-1`)
  (`RadialForceComponent.FireImpulse` (`self.RadialForce`))
  (`self.K2_DestroyActor`)
  (`|ExecutionSequence`
    (:`then_0`
      (message `/Game/Blueprint/BP_Interaction.Activate` (`self.FallingFloor`)))
    (:`then_1`
      (message `/Game/Blueprint/BP_Interaction.Activate` (`self.Platform`)))
    (:`then_2`
      (message `/Game/Blueprint/BP_Interaction.Activate` (`self.Vent`)))))

(fn `UserConstructionScript`)