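; Pressure plate puzzle blueprint that opens a door once the plate has been held down for a delay.
; Trigger overlap sinks the plate, starts a retriggerable delay, then raises the door if Triggered is still set.
; An overlap counter tracks actors on the trigger, so the door lowers and the plate resets only after the last one leaves.
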(event `self.Trigger.OnActorBeginOverlap`
  (params (OverlappedActor :type "Actor Object Reference") (OtherActor :type "Actor Object Reference"))
  (`|ExecutionSequence`
    (:`then_0`
      (set `self.Triggered` true)
      (`|ExecutionSequence`
        (:`then_0`
          (`KismetSystemLibrary.MoveComponentTo` (`self.PressurePlate`) (-1201.0 0.0 -145.0) (struct) false false 0.2))
        (:`then_1`
          (`KismetSystemLibrary.RetriggerableDelay` 5.0)
          (if (`self.Triggered`)
            (`KismetSystemLibrary.MoveComponentTo` (`self.Door`) (0.0 0.0 265.0) (struct) false false 0.8)))))
    (:`then_1`
      (bind _result (`/Engine/EditorBlueprintResources/StandardMacros.IncrementInt` (`self.CountActors`))))))

(event `self.Trigger.OnActorEndOverlap`
  (params (OverlappedActor :type "Actor Object Reference") (OtherActor :type "Actor Object Reference"))
  (bind _result (`/Engine/EditorBlueprintResources/StandardMacros.DecrementInt` (`self.CountActors`))
    (:`  `
      (if (== (`self.CountActors`) 0)
        (set `self.Triggered` false)
        (`|ExecutionSequence`
          (:`then_0`
            (`KismetSystemLibrary.MoveComponentTo` (`self.Door`) (0.0 0.0 0.0) (struct) false false 0.8))
          (:`then_1`
            (`KismetSystemLibrary.MoveComponentTo` (`self.PressurePlate`) (-1201.0 0.0 -140.0))))))))

(event `self.ReceiveBeginPlay`
  (`|ExecutionSequence`
    (:`then_0`
      (set `self.Triggered` false))
    (:`then_1`
      (set `self.CountActors` 0))))

(fn `UserConstructionScript`)