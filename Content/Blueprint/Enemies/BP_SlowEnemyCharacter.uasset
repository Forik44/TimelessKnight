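; Slow enemy character Blueprint that sets up its AI behavior when play begins.
; BeginPlay casts its controller to DefaulAIController and sets a fixed AI mode and type.
; Helper functions pick a random animation from a supplied array and update the attacking flag, then call the IsAttacking event.
; Tick and GetTurn are empty, and the DefaultSound playback is disconnected.
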(event `self.ReceiveBeginPlay`
  (bind _asdefaul_aicontroller (cast `/Game/AI/Controller/DefaulAIController` (`AIBlueprintHelperLibrary.GetAIController` self)))
  (`/Game/AI/Controller/DefaulAIController.SetAiModeAndType` _asdefaul_aicontroller true 1))

(event `self.ReceiveTick`
  (params (DeltaSeconds :type "Float (single-precision)")))

(fn `GetRandomAnimation`
  (params (Animations :type "Array of AnimMontage Object Reference"))
  (returns (Animation :type "AnimMontage Object Reference"))
  (return (`|GetArrayItem` Animations (`KismetMathLibrary.RandomInteger` (`KismetArrayLibrary.Array_Length` Animations)))))

(fn `GetTurn`)

(fn `SetIsAttacking`
  (params (`Is Attacking` :type Boolean))
  (set `self.IsAttacking` `Is Attacking`)
  (`self.IsAttackingEvent`))

(fn `UserConstructionScript`)