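; Spinning platform that yaws its cylinder on a looping artificial clock, which runs backwards while Rewinding.
; Each tick, actors in its Box are pushed linearly along the StaticMesh forward vector, using conveyor-style logic rather than following the rotation.
; The character is swept along unless an overlapping BP_Conveyor has control, and inherits the push as velocity when jumping or falling off.
; A disconnected Track material update is never run.
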(event `self.ReceiveTick`
  (params (DeltaSeconds :type "Float (single-precision)"))
  (bind _speed (`self.Speed`))
  (bind _cylinder (`self.Cylinder`))
  (bind _returnvalue (`KismetMathLibrary.GetForwardVector` (`SceneComponent.K2_GetComponentRotation` (`self.StaticMesh`))))
  (bind _returnvalue_2 (+ (* (`KismetMathLibrary.Conv_BoolToInt` (`self.Rewinding`)) -2) 1))
  (bind _returnvalue_3 (* _returnvalue_2 _speed))
  (bind _returnvalue_4 (+ (* _returnvalue_2 DeltaSeconds) (`self.ArtificialTime`)))
  (bind _returnvalue_5 (* _returnvalue (* DeltaSeconds _returnvalue_3)))
  (bind _output_get (set `self.ArtificialTime` (- _returnvalue_4 (* (`KismetMathLibrary.FFloor` (/ _returnvalue_4 (`self.Track Revolve Time`))) (`self.Track Revolve Time`)))))
  (`SceneComponent.K2_SetRelativeRotation` _cylinder (`KismetMathLibrary.MakeRotator` (.roll (`SceneComponent.RelativeRotation` _cylinder)) (.pitch (`SceneComponent.RelativeRotation` _cylinder)) (* (* _output_get 360.0) _speed)) false false)
  (set `self.CanControl` true)
  (for _array_element (`PrimitiveComponent.GetOverlappingActors` (`self.Box`) null)
    (bind _ascharacter (cast `Character` _array_element)
      (:`then`
        (set `self.Character` _ascharacter))
      (:`CastFailed`
        (bind _asbp_conveyor (cast `/Game/Blueprint/BP_Conveyor` _array_element)
          (:`then`
            (if (or (and (`PrimitiveComponent.IsOverlappingActor` (`/Game/Blueprint/BP_Conveyor.Box` _asbp_conveyor) (`self.Character`)) (`/Game/Blueprint/BP_Conveyor.CanControl` _asbp_conveyor)) (`/Game/Blueprint/BP_Conveyor.Controlling` _asbp_conveyor))
              (set `self.CanControl` false)))
          (:`CastFailed`
            (`self.K2_AddActorWorldOffset` _array_element _returnvalue_5 false false))))))
  (bind _asfpcharacter (cast `FPCharacter` (`self.Character`)))
  (if (`self.CanControl`)
    (bind _charactermovement (`Character.CharacterMovement` _asfpcharacter))
    (if (and (or (`Character.bWasJumping` _asfpcharacter) (`NavMovementComponent.IsFalling` _charactermovement)) (`self.Controlling`))
      (set `MovementComponent.Velocity` (+ (`MovementComponent.Velocity` _charactermovement) (* _returnvalue _returnvalue_3)) _charactermovement)
      (set `self.CanControl` false)
      (set `self.Controlling` false :!label _label)
      (else
        (set `self.Controlling` true)
        (if (`PrimitiveComponent.IsOverlappingActor` (`self.Box`) (`self.Character`))
          (`self.K2_AddActorWorldOffset` (`self.Character`) _returnvalue_5 true false)
          (set `self.CanControl` (`PrimitiveComponent.IsOverlappingActor` (`self.Box`) (`self.Character`)))
          (else
            (goto _label)))))))

(fn `UserConstructionScript`
  (`parent.UserConstructionScript`))