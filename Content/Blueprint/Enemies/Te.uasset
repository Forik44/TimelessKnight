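; Te is an input-driven Blueprint that appears to be a test harness for time reversal on an interactive ramp.
; Holding the left mouse button starts reversal on the TimeSystemComponent of the first BP_InteractiveRamp found, releasing stops it, and both print a debug message.
; Right mouse and key 1 only gather slow enemy or Te actors without acting on them, leaving those bindings unfinished.
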(event `Key|LeftMouseButton`
  (params (Key :type "Key Structure"))
  (:`Pressed`
    (bind _outactors (`GameplayStatics.GetAllActorsOfClass` "/Game/Blueprint/BP_InteractiveRamp.BP_InteractiveRamp_C"))
    (`TimeSystemComponent.StartRevers` (`self.GetComponentByClass` (`|GetArrayItem` _outactors) "/Script/STimelessKnight.TimeSystemComponent"))
    (`KismetSystemLibrary.PrintString` "Hello" :!label _label))
  (:`Released`
    (bind _outactors_2 (`GameplayStatics.GetAllActorsOfClass` "/Game/Blueprint/BP_InteractiveRamp.BP_InteractiveRamp_C"))
    (`TimeSystemComponent.StopRevers` (`self.GetComponentByClass` (`|GetArrayItem` _outactors_2) "/Script/STimelessKnight.TimeSystemComponent"))
    (goto _label)))

(event `Key|RightMouseButton`
  (params (Key :type "Key Structure"))
  (:`Pressed`
    (bind _outactors (`GameplayStatics.GetAllActorsOfClass` "/Game/Blueprint/Enemies/BP_SlowEnemyCharacter.BP_SlowEnemyCharacter_C"))
    (for _ _outactors
      _))
  (:`Released`
    (bind _outactors_2 (`GameplayStatics.GetAllActorsOfClass` "/Game/Blueprint/Enemies/BP_SlowEnemyCharacter.BP_SlowEnemyCharacter_C"))
    (for _ _outactors_2
      _)))

(event `Key|One`
  (params (Key :type "Key Structure"))
  (:`Pressed`
    (bind _outactors (`GameplayStatics.GetAllActorsOfClass` "Te_C")))
  (:`Released`
    (bind _outactors_2 (`GameplayStatics.GetAllActorsOfClass` "Te_C"))))

(fn `UserConstructionScript`)