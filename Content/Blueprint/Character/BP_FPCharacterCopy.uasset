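; First-person player character Blueprint that adds conveyor rewinding, interaction and pause menu toggling.
; The reverse-object press event traces from the camera and sets a hit BP_Conveyor rewinding, with a looping timer applying mana changes until release.
; E sends InteractMessage to a short-range trace hit, and Escape toggles the pause widget.
; Tick traces ahead to flag the crosshair as interactable over items, enemies or conveyors.
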(event `OnReversObjectReleasedEvent`
  (bind _pressedconveyor (`self.PressedConveyor`))
  (`/Engine/EditorBlueprintResources/StandardMacros.IsValid` _pressedconveyor
    (:`Is Valid`
      (if (`/Game/Blueprint/BP_Conveyor.Rewinding` _pressedconveyor)
        (set `/Game/Blueprint/BP_Conveyor.Rewinding` false _pressedconveyor)
        (`KismetSystemLibrary.K2_ClearAndInvalidateTimerHandle` (`self.ManaConveyorTimer`))))))

(event `self.ReceiveBeginPlay`
  (add `self.OnReversObjectPressed` (delegate `OnReversObjectPressedEvent`))
  (add `self.OnReversObjectReleased` (delegate `OnReversObjectReleasedEvent`)))

(event `OnReversObjectPressedEvent`
  (bind _camera (`self.Camera`))
  (bind _returnvalue (`SceneComponent.K2_GetComponentLocation` _camera))
  (bind _outhit (`KismetSystemLibrary.LineTraceSingleForObjects` _returnvalue (+ _returnvalue (* (`SceneComponent.GetForwardVector` _camera) 1000.0)) (`|MakeArray` "ObjectTypeQuery2" :!type "EObjectTypeQuery Enum") true))
  (bind _asbp_conveyor (cast `/Game/Blueprint/BP_Conveyor` (`.HitActor` (`GameplayStatics.BreakHitResult` _outhit))))
  (set `self.PressedConveyor` _asbp_conveyor)
  (if (not (`/Game/Blueprint/BP_Conveyor.Rewinding` _asbp_conveyor))
    (set `/Game/Blueprint/BP_Conveyor.Rewinding` true _asbp_conveyor)
    (bind _returnvalue_2 (`KismetSystemLibrary.K2_SetTimerDelegate` (delegate `OnManaChangedOtherObject`) 1.0 true -1.0))
    (set `self.ManaConveyorTimer` _returnvalue_2)))

(event `OnManaChangedOtherObject`
  (`self.ChangeManaRTOtherObject` (`self.ManaConveyorTimer`) (`self.ConveyorMana`)))

(event `Key|Escape` :paused true
  (params (Key :type "Key Structure"))
  (bind _mainwidjet (`self.MainWidjet`))
  (:`Pressed`
    (if (`self.IsPause`)
      (`/Game/Blueprint/BP_MainWidjet.HidePause` _mainwidjet)
      (set `self.IsPause` false)
      (else
        (`/Game/Blueprint/BP_MainWidjet.ShowPause` _mainwidjet)
        (set `self.IsPause` true)))))

(event `Key|E`
  (params (Key :type "Key Structure"))
  (bind _camera (`self.Camera`))
  (bind _returnvalue (`SceneComponent.K2_GetComponentLocation` _camera))
  (:`Pressed`
    (bind (_outhit _returnvalue_2) (`KismetSystemLibrary.LineTraceSingleForObjects` :`Start` _returnvalue :`End` (+ _returnvalue (* (`SceneComponent.GetForwardVector` _camera) 200.0)) :`ObjectTypes` (`|MakeArray` "ObjectTypeQuery2" :!type "EObjectTypeQuery Enum") :`bTraceComplex` true :`DrawDebugType` "ForDuration"))
    (if _returnvalue_2
      (message `/Game/Blueprint/BP_Interaction.Interact` (`.HitActor` (`GameplayStatics.BreakHitResult` _outhit))))))

(event `self.ReceiveTick`
  (params (DeltaSeconds :type "Float (single-precision)"))
  (bind _camera (`self.Camera`))
  (bind _returnvalue (`SceneComponent.K2_GetComponentLocation` _camera))
  (bind _bp_crosshair (`/Game/Blueprint/BP_MainWidjet.BP_Crosshair` (`self.MainWidjet`)))
  (bind _outhit (`KismetSystemLibrary.LineTraceSingleForObjects` _returnvalue (+ _returnvalue (* (`SceneComponent.GetForwardVector` _camera) 1000.0)) (`|MakeArray` "ObjectTypeQuery2" "ObjectTypeQuery3" "ObjectTypeQuery4" :!type "EObjectTypeQuery Enum") true))
  (cast `InteractiveItem` (`.HitActor` (`GameplayStatics.BreakHitResult` _outhit))
    (:`then`
      (set `/Game/Blueprint/BP_Crosshair.canInteract` true _bp_crosshair))
    (:`CastFailed`
      (cast `DefaultEnemyCharacter` (`.HitActor` (`GameplayStatics.BreakHitResult` _outhit))
        (:`then`
          (set `/Game/Blueprint/BP_Crosshair.canInteract` true _bp_crosshair))
        (:`CastFailed`
          (cast `/Game/Blueprint/BP_Conveyor` (`.HitActor` (`GameplayStatics.BreakHitResult` _outhit))
            (:`then`
              (set `/Game/Blueprint/BP_Crosshair.canInteract` true _bp_crosshair))
            (:`CastFailed`
              (set `/Game/Blueprint/BP_Crosshair.canInteract` false _bp_crosshair))))))))

(fn `UserConstructionScript`)