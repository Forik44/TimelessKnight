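; BP_KillArea is a box-shaped area that calls ChangeXP with zero on a first-person player character inside it.
; Each Tick it polls the box's overlapping actors and stores each one that casts to Character.
; It then checks that the stored BP_FPCharacter's capsule overlaps the box before making the call through an FPCharacter cast.
; Detection relies on per-frame polling, with no overlap events.
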(event `self.ReceiveTick`
  (params (DeltaSeconds :type "Float (single-precision)"))
  (for _array_element (`PrimitiveComponent.GetOverlappingActors` (`self.BoxC`) null)
    (bind _ascharacter (cast `Character` _array_element))
    (set `self.Character` _ascharacter))
  (bind _asbp_fpcharacter (cast `/Game/Blueprint/Character/BP_FPCharacter` (`self.Character`)))
  (if (`PrimitiveComponent.IsOverlappingComponent` (`self.BoxC`) (`Character.CapsuleComponent` _asbp_fpcharacter))
    (bind _asfpcharacter (cast `FPCharacter` (`self.Character`)))
    (`FPCharacter.ChangeXP` _asfpcharacter 0.0)))

(fn `UserConstructionScript`)