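; LockedDoor is a riddle door Blueprint that moves open and closed through Activate and Deactivate events.
; A DoorAnimation timeline lerps the Door component's relative location from the origin to UpState without sweeping, and reverses on deactivation.
; Both events play DoorSound from the start, and BeginPlay stops that sound so it is silent until triggered.
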(event `/Game/Blueprint/BP_Interaction.Activate`
  (`AudioComponent.Play` (`self.DoorSound`) 0.0)
  (bind (_direction _lerp) (`Timeline|DoorAnimation` :!label _label)
    (:`Update`
      (`SceneComponent.K2_SetRelativeLocation` (`self.Door`) (`KismetMathLibrary.VLerp` (0.0 0.0 0.0) (`self.UpState`) _lerp) false false))))

(event `/Game/Blueprint/BP_Interaction.Deactivate`
  (`AudioComponent.Play` (`self.DoorSound`) 0.0)
  (goto _label :!via `Reverse`))

(event `self.ReceiveBeginPlay`
  (`AudioComponent.Stop` (`self.DoorSound`)))

(fn `UserConstructionScript`)